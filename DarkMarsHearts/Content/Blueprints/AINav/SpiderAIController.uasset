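; AI controller that moves an AiEntity_BP pawn across surfaces using a SpiderNavigation node graph, driven by the SpiderBT behavior tree.
; Move finds a path between nodes and randomly jitters its waypoints to vary the route.
; Tick rotates the pawn to face each waypoint aligned to the node normal, then offsets it forward without sweeping and signals completion near the destination.
; A looping timer refreshes the local waypoint while moving.
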(event `OnFindPathTick`
  (if (`self.MustMove`)
    (`self.UpdateLocalMoveDestination`)
    (if (not (`self.LocalPathFound`))
      (set `self.MustMove` false))))

(event `self.ReceiveBeginPlay`
  (bind _returnvalue (`self.K2_GetPawn`))
  (`|ExecutionSequence`
    (:`then_0`
      (bind _outactors (`GameplayStatics.GetAllActorsOfClass` "/Script/SpiderNavigation.SpiderNavigation"))
      (if (> (`KismetArrayLibrary.Array_Length` _outactors) 0)
        (set `self.Navigation` (`|GetArrayItem` _outactors))
        (`KismetSystemLibrary.K2_SetTimerDelegate` (delegate `OnFindPathTick`) (`self.UpdateLocalDestinationInterval`) true)
        (else
          (`KismetSystemLibrary.PrintString` "No navigation actor for movement" true true (struct :`R` 1.0 :`B` 0.14292 :`A` 1.0)))))
    (:`then_1`
      (`self.UseBlackboard` "/SpiderNavigation/Behavior/SpiderBB.SpiderBB")
      (`/Engine/EditorBlueprintResources/StandardMacros.IsValid` _returnvalue
        (:`Is Valid`
          (bind _returnvalue_2 (`SpiderNavigation.FindClosestNodeLocation` (`self.Navigation`) (`self.K2_GetActorLocation` _returnvalue)))
          (if (`AIBlueprintHelperLibrary.IsValidAILocation` _returnvalue_2)
            (`BlackboardComponent.SetValueAsVector` (`AIBlueprintHelperLibrary.GetBlackboard` self) (`self.HomeLocation`) _returnvalue_2)
            (`self.RunBehaviorTree` "/SpiderNavigation/Behavior/SpiderBT.SpiderBT")))))))

(event `self.ReceiveTick`
  (params (DeltaSeconds :type "Float (single-precision)"))
  (bind _returnvalue (`self.K2_GetPawn`))
  (bind _pawnref (`self.PawnRef`))
  (bind _pawnref_2 (`self.PawnRef`))
  (bind _pawnref_3 (`self.PawnRef`))
  (bind _pawnref_4 (`self.PawnRef`))
  (`/Engine/EditorBlueprintResources/StandardMacros.IsValid` (`self.PawnRef`)
    (:`Is Valid`
      _)
    (:`Is Not Valid`
      (bind _asai_entity_bp (cast `/Game/Blueprints/Entities/AiEntity_BP` (`self.K2_GetPawn`)))
      (set `self.PawnRef` _asai_entity_bp)))
  (`|ExecutionSequence`
    (:`then_0`
      (`/Engine/EditorBlueprintResources/StandardMacros.IsValid` _pawnref_2
        (:`Is Valid`
          ;[1 1 1] Check finish
          (if (< (`KismetMathLibrary.VSize` (- (`self.K2_GetActorLocation` _pawnref_2) (`self.MoveDestination`))) (* (`/Game/Blueprints/Entities/AiEntity_BP.MoveSpeed` _pawnref_2) 0.2))
            (set `self.MustMove` false)
            (`self.MovementComplete` true)))))
    (:`then_1`
      ;[1 1 1] Rotation
      (if (`self.MustRotate`)
        (if (!= (`self.K2_GetActorRotation` (`self.PawnRef`)) (`self.RotationDestination`) :`ErrorTolerance` 0.01)
          (if (`SceneComponent.IsSimulatingPhysics` (`/Game/Blueprints/Entities/Entity_BP.Box` _pawnref) "None")
            _
            (elif (not (or (== (`/Game/Blueprints/Entities/Entity_BP.Durability` _pawnref_3) 0.0) (`/Game/Blueprints/Entities/Entity_BP.Connected` _pawnref_3)))
              (`self.K2_SetActorRotation` (`self.K2_GetPawn`) (`KismetMathLibrary.RInterpTo` (`self.K2_GetActorRotation` (`self.K2_GetPawn`)) (`self.RotationDestination`) DeltaSeconds (`/Game/Blueprints/Entities/AiEntity_BP.RotateSpeed` _pawnref)) false)))
          (else
            (set `self.MustRotate` false)))))
    (:`then_2`
      ;[1 1 1] Move
      (if (and (not (`self.MustRotate`)) (`self.MustMove`) (`self.MustMoveLocal`))
        (set `self.NormalToDestinationBeforeMove` (`self.GetNormalToLocalDestination`))
        (if (not (or (== (`/Game/Blueprints/Entities/Entity_BP.Durability` _pawnref_4) 0.0) (`/Game/Blueprints/Entities/Entity_BP.Connected` _pawnref_4)))
          (`self.K2_AddActorWorldOffset` _returnvalue (* (`self.GetActorForwardVector` _returnvalue) (* DeltaSeconds (`/Game/Blueprints/Entities/AiEntity_BP.MoveSpeed` _pawnref_4))) false false)
          (if (or (!= (`self.GetNormalToLocalDestination`) (`self.NormalToDestinationBeforeMove`) :`ErrorTolerance` 0.1) (< (`KismetMathLibrary.VSize` (- (`self.K2_GetActorLocation` (`self.K2_GetPawn`)) (`self.LocalMoveDestination`))) (* (`/Game/Blueprints/Entities/AiEntity_BP.MoveSpeed` _pawnref_4) 0.05)))
            (`KismetArrayLibrary.Array_Remove` (`self.CurrentPath`))
            (`self.UpdateLocalMoveDestination`)))))))

(fn `Move`
  (params (Destination :type "Vector Structure"))
  (bind _returnvalue (`self.K2_GetPawn`))
  (bind _returnvalue_2 (`self.K2_GetPawn`))
  (bind _returnvalue_3 (`SpiderNavigation.FindClosestNodeLocation` (`self.Navigation`) Destination))
  (if (not (== _returnvalue_3 (`self.MoveDestination`)))
    (bind _output_get (set `self.MoveDestination` _returnvalue_3))
    (bind _asai_entity_bp (cast `/Game/Blueprints/Entities/AiEntity_BP` _returnvalue_2)
      (:`then`
        (set `/Game/Blueprints/Entities/AiEntity_BP.MoveDestinationRef` _output_get _asai_entity_bp))
      (:`CastFailed`
        _))
    (bind (_bfoundcompletepath _returnvalue_4) (`SpiderNavigation.FindPath` (`self.Navigation`) (`self.K2_GetActorLocation` _returnvalue_2) _output_get))
    (bind _output_get_2 (set `self.CurrentPath` _returnvalue_4))
    (for (_array_element _array_index) _output_get_2
      (`KismetArrayLibrary.Array_Set` _output_get_2 _array_index (+ _array_element (* (`self.GetActorRightVector` _returnvalue) (`KismetMathLibrary.RandomFloatInRange` -100.0 100.0)) (0.0 0.0 0.0) (* (`self.GetActorUpVector` _returnvalue) (`KismetMathLibrary.RandomFloatInRange` -10.0 10.0)))))
    (`KismetArrayLibrary.Array_Remove` _output_get_2)
    (`self.UpdateLocalMoveDestination`)
    (if (`self.LocalPathFound`)
      (set `self.MustMove` true))))

(fn `UpdateLocalMoveDestination`
  (if (> (`KismetArrayLibrary.Array_Length` (`self.CurrentPath`)) 0)
    (bind _output_get (set `self.LocalMoveDestination` (`|GetArrayItem` (`self.CurrentPath`))))
    (bind _returnvalue (`SpiderNavigation.FindClosestNodeNormal` (`self.Navigation`) _output_get))
    (set `self.MoveNormal` _returnvalue)
    (set `self.LocalPathFound` true)
    (set `self.MustMoveLocal` true)
    (`self.UpdateRotationParams`)
    (else
      (set `self.LocalPathFound` false)
      (set `self.MustMoveLocal` false)))
  ;[1 1 1] Debug
  (for _array_element (`self.CurrentPath`)
    _)
  (bind _returnvalue_2 (`SpiderNavigation.FindClosestNodeLocation` (`self.Navigation`) (`self.MoveDestination`))))

(fn `UpdateRotationParams`
  (set `self.RotationBeforeMove` (`self.K2_GetActorRotation` (`self.K2_GetPawn`)))
  (set `self.RotationDestination` (`KismetMathLibrary.MakeRotFromXZ` (- (`self.LocalMoveDestination`) (`self.K2_GetActorLocation` (`self.K2_GetPawn`))) (`self.MoveNormal`)))
  (set `self.MustRotate` (!= (`self.RotationDestination`) (`self.RotationBeforeMove`) :`ErrorTolerance` 0.01)))

(fn `UserConstructionScript`)