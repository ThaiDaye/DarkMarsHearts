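; Debug Blueprint for spider AI navigation that loads, builds and visualizes a custom nav grid.
; One second after BeginPlay it gathers all SpiderNavGridBuilder actors and tries LoadGrid, building through every builder if loading fails.
; NumPad 2 forces a rebuild and NumPad 1 draws the grid connections.
; A distance-based auto-rebuild event exists, but its looping timer is disconnected.
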(event `RebuildGridAuto`
  (if (>= (`KismetMathLibrary.VSize` (- (`self.K2_GetActorLocation` (`|GetArrayItem` (`self.SpiderNavGridBuilders`))) (`self.LastLoc`))) (`self.GridBuildDistance`))
    (bind _returnvalue (`self.LoadGrid` :!label _label))
    (if (not _returnvalue)
      (for _array_element (`self.SpiderNavGridBuilders`) :!label _label_2
        (`SpiderNavGridBuilder.BuildGrid` _array_element))
      (`KismetSystemLibrary.PrintString` "Custom Nav Grid has been built" true true (struct :`G` 1.0 :`B` 0.187617 :`A` 1.0) 1.0)
      (set `self.LastLoc` (`self.K2_GetActorLocation` _array_element)))))

(event `self.ReceiveBeginPlay`
  (`KismetSystemLibrary.Delay` 1.0)
  (bind _outactors (`GameplayStatics.GetAllActorsOfClass` "/Script/SpiderNavigation.SpiderNavGridBuilder"))
  (if (> (`KismetArrayLibrary.Array_Length` _outactors) 0)
    (set `self.SpiderNavGridBuilders` _outactors)
    (`self.BuildGridInit`)))

(event `BuildGridInit`
  (goto _label))

(event `Key|NumPadOne`
  (params (Key :type "Key Structure"))
  (:`Pressed`
    (`self.DrawDebugRelations`)))

(event `Key|NumPadTwo`
  (params (Key :type "Key Structure"))
  (:`Pressed`
    (goto _label_2)))

(fn `UserConstructionScript`)