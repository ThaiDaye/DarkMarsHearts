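; Spider navigation grid builder Blueprint that maintains its actor blacklist for the player and physics-driven entities.
; On BeginPlay it runs the parent logic, caches the first PlayerEntity_BP and fills the blacklist.
; A looping timer then rebuilds the list every few seconds from all Entity_BP actors whose Box simulates physics, always re-adding the player.
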(event `self.ReceiveBeginPlay`
  (`parent.ReceiveBeginPlay`)
  (bind _outactors (`GameplayStatics.GetAllActorsOfClass` "/Game/Blueprints/Entities/PlayerEntity_BP.PlayerEntity_BP_C"))
  (set `self.PlayerRef` (`|GetArrayItem` _outactors))
  (`self.AddtoBlackList`)
  (`KismetSystemLibrary.K2_SetTimerDelegate` (delegate `AddtoBlackList`) 3.0 true))

(event `AddtoBlackList`
  (`KismetArrayLibrary.Array_Clear` (`self.ActorsBlackList`))
  (bind _outactors (`GameplayStatics.GetAllActorsOfClass` "/Game/Blueprints/Entities/Entity_BP.Entity_BP_C"))
  (for _array_element _outactors
    (if (`SceneComponent.IsSimulatingPhysics` (`/Game/Blueprints/Entities/Entity_BP.Box` _array_element) "None")
      (`KismetArrayLibrary.Array_Add` (`self.ActorsBlackList`) _array_element)))
  (`KismetArrayLibrary.Array_Add` (`self.ActorsBlackList`) (`self.PlayerRef`)))

(fn `UserConstructionScript`)