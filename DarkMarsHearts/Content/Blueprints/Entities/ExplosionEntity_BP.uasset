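; Short-lived explosion entity that heats, damages and pushes nearby entities, then destroys itself.
; On BeginPlay it derives Temperature from Durability, explodes after a brief delay and lingers before removal.
; A sphere trace gathers Pawn-type entities, skips temperature entities, and applies emitted heat and Durability-based burn damage to the rest.
; Surviving physics-simulated entities receive an outward, slightly upward velocity impulse, scaled by Durability and trace hit distance.
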(event `self.ReceiveBeginPlay`
  (`parent.ReceiveBeginPlay`)
  (set `self.Temperature` (* (`self.Durability`) 1.5))
  (`KismetSystemLibrary.Delay` 0.1)
  (`self.Explosion`)
  (`KismetSystemLibrary.Delay` 2.0)
  (`self.K2_DestroyActor`))

(event `Explosion`
  (bind _sphere (`self.Sphere`))
  (bind _returnvalue (`SceneComponent.K2_GetComponentLocation` _sphere))
  (bind _returnvalue_2 (`KismetMathLibrary.VSize` (* (`SceneComponent.K2_GetComponentScale` _sphere) (`SphereComponent.SphereRadius` _sphere))))
  (bind _outhits (`KismetSystemLibrary.SphereTraceMultiForObjects` _returnvalue _returnvalue _returnvalue_2 (`|MakeArray` "ObjectTypeQuery3" :!type "EObjectTypeQuery Enum")))
  (for _array_element _outhits
    (bind (_bblockinghit _binitialoverlap _time _distance _location _impactpoint _normal _impactnormal _physmat _hitactor) (`GameplayStatics.BreakHitResult` _array_element))
    (bind _asentity_bp (cast `/Game/Blueprints/Entities/Entity_BP` _hitactor))
    (cast `/Game/Blueprints/Entities/TemperatureEntity_BP` _hitactor
      (:`CastFailed`
        (`self.EmitTemperature` _asentity_bp 1.2)
        (`self.ReduceDurability` _asentity_bp (* (`self.Durability`) 0.5) true false false false (0.0 0.0 0.0))
        (`/Engine/EditorBlueprintResources/StandardMacros.IsValid` _asentity_bp
          (:`Is Valid`
            (bind _box (`/Game/Blueprints/Entities/Entity_BP.Box` _asentity_bp))
            (if (`SceneComponent.IsSimulatingPhysics` _box "None")
              (`PrimitiveComponent.AddImpulse` _box (* (+ (* (`KismetMathLibrary.Conv_RotatorToVector` (`KismetMathLibrary.FindLookAtRotation` (`self.K2_GetActorLocation`) _impactpoint)) 100.0) (* (`KismetMathLibrary.GetUpVector` (struct)) 50.0)) (`KismetMathLibrary.FClamp` (* (* (`self.Durability`) 0.25) (`KismetMathLibrary.Lerp` 1.0 0.0 (/ _distance _returnvalue_2))))) "None" true))))))))

(fn `UserConstructionScript`
  (`parent.UserConstructionScript`))