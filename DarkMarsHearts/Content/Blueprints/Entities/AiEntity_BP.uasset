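; AI creature entity, run by a spider behavior tree, that crawls surfaces and periodically leaps toward its move destination.
; Leaping or being grabbed switches its box to physics and, after a short delay, opens a gate for hit events.
; Hitting a non-entity while unfrozen, unchained and not at zero durability respawns it as a fresh AI copy, carrying over state, fire and footprints, then destroys the original.
; Footprint spawning is disabled.
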(event `LeaveFootprint`
  ;[1 0 0.09374] disabled for now
)

(event `VelocityCheck`
  (set `self.AiVelocity` (`KismetMathLibrary.VSize` (- (`self.K2_GetActorLocation`) (`self.LastPosDEBUG`))))
  (set `self.LastPosDEBUG` (`self.K2_GetActorLocation`)))

(event `self.ReceiveBeginPlay`
  (`parent.ReceiveBeginPlay`)
  (`KismetSystemLibrary.K2_SetTimerDelegate` (delegate `LeapEvent`) (`KismetMathLibrary.RandomFloatInRange` 6.0 12.0) true)
  (`KismetSystemLibrary.K2_SetTimerDelegate` (delegate `LeaveFootprint`) 3.0 true)
  (`KismetSystemLibrary.K2_SetTimerDelegate` (delegate `VelocityCheck`) 1.0 true)
  (`SceneComponent.K2_AttachToComponent` (`self.MainMesh`) (`self.SpringArm`) "None" "KeepRelative" "KeepRelative" "KeepRelative" true))

(event `LeapEvent`
  (bind _returnvalue (`self.K2_GetActorLocation`))
  (bind (_returnvalue_location _returnvalue_rotation _returnvalue_scale) (`KismetMathLibrary.BreakTransform` (`self.GetTransform`)))
  (bind _fireref (`self.FireRef`))
  (bind _leapstrength (`self.LeapStrength`))
  (bind _box (`self.Box`))
  (bind _returnvalue_2 (`KismetMathLibrary.FindLookAtRotation` (`self.K2_GetActorLocation`) (`self.MoveDestinationRef`)))
  (if (not (or (`self.Connected`) (== (`self.Durability`) 0.0)))
    (bind _outhit (`KismetSystemLibrary.SphereTraceSingleForObjects` _returnvalue _returnvalue 50.0 (`|MakeArray` "ObjectTypeQuery1" "ObjectTypeQuery3" :!type "EObjectTypeQuery Enum")))
    (if (`GameplayStatics.BreakHitResult` _outhit)
      (`KismetSystemLibrary.PrintString` "LEAP" true true (struct :`R` 1.0 :`G` 0.349428 :`A` 1.0))
      (`PrimitiveComponent.SetCollisionResponseToChannel` _box "ECC_WorldStatic" "ECR_Block")
      (`PrimitiveComponent.SetCollisionResponseToChannel` _box "ECC_WorldDynamic" "ECR_Block")
      (`PrimitiveComponent.SetSimulatePhysics` _box true)
      (`PrimitiveComponent.AddImpulse` _box (+ (* (`KismetMathLibrary.Conv_RotatorToVector` _returnvalue_2) _leapstrength) (`KismetMathLibrary.MakeVector` 0.0 0.0 _leapstrength)) "None" true)
      (`self.K2_SetActorRotation` _returnvalue_2)
      (if (`self.OnFire`)
        (`self.ReduceDurability` 20.0))
      (`KismetSystemLibrary.Delay` (`KismetMathLibrary.RandomFloatInRange` 0.0 1.0) :!label _label)
      (goto _label_2 :!via `Open`)
      (else
        (`KismetSystemLibrary.PrintString` "LEAP ATTEMPT" true true (struct :`R` 0.427083 :`G` 0.149235 :`A` 1.0))))))

(event `GrabEvent`
  (bind _box (`self.Box`))
  (`PrimitiveComponent.SetCollisionResponseToChannel` _box "ECC_WorldStatic" "ECR_Block")
  (`PrimitiveComponent.SetCollisionResponseToChannel` _box "ECC_WorldDynamic" "ECR_Block")
  (`PrimitiveComponent.SetSimulatePhysics` _box true)
  (goto _label))

(event `self.ReceiveHit`
  (params (MyComp :type "PrimitiveComponent Object Reference") (Other :type "Actor Object Reference") (OtherComp :type "PrimitiveComponent Object Reference") (bSelfMoved :type Boolean) (HitLocation :type "Vector Structure") (HitNormal :type "Vector Structure") (NormalImpulse :type "Vector Structure") (Hit :type "HitResult Structure (by ref)"))
  (bind (_returnvalue_location _returnvalue_rotation _returnvalue_scale) (`KismetMathLibrary.BreakTransform` (`self.GetTransform`)))
  (bind _fireref (`self.FireRef`))
  (`parent.ReceiveHit` MyComp Other OtherComp bSelfMoved HitLocation HitNormal NormalImpulse Hit)
  (`/Engine/EditorBlueprintResources/StandardMacros.Gate` true :!label _label_2
    (:`Exit`
      (cast `/Game/Blueprints/Entities/Entity_BP` Other
        (:`CastFailed`
          (if (`self.IsFrozen`)
            _
            (elif (== (`self.Durability`) 0.0)
              _
              (elif (`KismetArrayLibrary.Array_IsValidIndex` (`self.ChainRef`))
                (`/Engine/EditorBlueprintResources/StandardMacros.DoOnce` false
                  (:`Completed`
                    (`KismetSystemLibrary.PrintString` "AI Cant Reattach to wall, Due to Chain")))
                (else
                  (`KismetSystemLibrary.PrintString` "AI Reattach to walls")
                  (bind _returnvalue (`AIBlueprintHelperLibrary.SpawnAIFromClass` "AiEntity_BP_C" "/SpiderNavigation/Behavior/SpiderBT.SpiderBT" _returnvalue_location _returnvalue_rotation true))
                  (`self.SetActorScale3D` _returnvalue _returnvalue_scale)
                  (bind _asai_entity_bp (cast `/Game/Blueprints/Entities/AiEntity_BP` _returnvalue))
                  (set `/Game/Blueprints/Entities/AiEntity_BP.LeapingDEBUG` (not (`self.LeapingDEBUG`)) _asai_entity_bp)
                  (set `/Game/Blueprints/Entities/Entity_BP.Durability` (`self.Durability`) _asai_entity_bp)
                  (set `/Game/Blueprints/Entities/Entity_BP.Connected` (`self.Connected`) _asai_entity_bp)
                  (set `/Game/Blueprints/Entities/Entity_BP.Density` (`self.Density`) _asai_entity_bp)
                  (set `/Game/Blueprints/Entities/Entity_BP.MaxDurability` (`self.MaxDurability`) _asai_entity_bp)
                  (set `/Game/Blueprints/Entities/Entity_BP.Temperature` (`self.Temperature`) _asai_entity_bp)
                  (bind _output_get (set `/Game/Blueprints/Entities/Entity_BP.OnFire` (`self.OnFire`) _asai_entity_bp))
                  (set `/Game/Blueprints/Entities/Entity_BP.Wetness` (`self.Wetness`) _asai_entity_bp)
                  (set `/Game/Blueprints/Entities/AiEntity_BP.BaseMoveSpeed` (`self.BaseMoveSpeed`) _asai_entity_bp)
                  (set `/Game/Blueprints/Entities/AiEntity_BP.MoveSpeed` (`self.MoveSpeed`) _asai_entity_bp)
                  (set `/Game/Blueprints/Entities/Entity_BP.IsFrozen` (`self.IsFrozen`) _asai_entity_bp)
                  (set `/Game/Blueprints/Entities/Entity_BP.LastHitLoc` (`self.LastHitLoc`) _asai_entity_bp)
                  (set `/Game/Blueprints/Entities/Entity_BP.TotalBurnDamage` (`self.TotalBurnDamage`) _asai_entity_bp)
                  (set `/Game/Blueprints/Entities/AiEntity_BP.FootstepEntities` (`self.FootstepEntities`) _asai_entity_bp)
                  (set `/Game/Blueprints/Entities/Entity_BP.Name` (`self.Name`) _asai_entity_bp)
                  (set `/Game/Blueprints/Entities/Entity_BP.TemperaturePerSecFreeze` (`self.TemperaturePerSecFreeze`) _asai_entity_bp)
                  (set `/Game/Blueprints/Entities/Entity_BP.TemperaturePerSecMelt` (`self.TemperaturePerSecMelt`) _asai_entity_bp)
                  (set `/Game/Blueprints/Entities/Entity_BP.IsFrozenPerSec` (`self.IsFrozenPerSec`) _asai_entity_bp)
                  (set `/Game/Blueprints/Entities/Entity_BP.Friction` (`self.Friction`) _asai_entity_bp)
                  (set `/Game/Blueprints/Entities/Entity_BP.Bounciness` (`self.Bounciness`) _asai_entity_bp)
                  (set `/Game/Blueprints/Entities/Entity_BP.Bouyancy` (`self.Bouyancy`) _asai_entity_bp)
                  (set `/Game/Blueprints/Entities/Entity_BP.HydroReaction` (`self.HydroReaction`) _asai_entity_bp)
                  (set `/Game/Blueprints/Entities/Entity_BP.WetnessType` (`self.WetnessType`) _asai_entity_bp)
                  (set `/Game/Blueprints/Entities/Entity_BP.SolidType` (`self.SolidType`) _asai_entity_bp)
                  (set `/Game/Blueprints/Entities/Entity_BP.GasStorageCapacity` (`self.GasStorageCapacity`) _asai_entity_bp)
                  (set `/Game/Blueprints/Entities/Entity_BP.GasStorageMax` (`self.GasStorageMax`) _asai_entity_bp)
                  (set `/Game/Blueprints/Entities/Entity_BP.GasStorageType` (`self.GasStorageType`) _asai_entity_bp)
                  (set `/Game/Blueprints/Entities/Entity_BP.LiquidStorageCapacity` (`self.LiquidStorageCapacity`) _asai_entity_bp)
                  (set `/Game/Blueprints/Entities/Entity_BP.LiquidStorageMax` (`self.LiquidStorageMax`) _asai_entity_bp)
                  (set `/Game/Blueprints/Entities/Entity_BP.LiquidStorageType` (`self.LiquidStorageType`) _asai_entity_bp)
                  (if _output_get
                    (`self.K2_AttachToActor` _fireref _asai_entity_bp "None" "KeepRelative" "KeepRelative" "KeepRelative" true)
                    (bind _output_get_2 (set `/Game/Blueprints/Entities/Entity_BP.FireRef` _fireref _asai_entity_bp))
                    (set `/Game/Blueprints/Entities/FireEntity_BP.Host` _asai_entity_bp _output_get_2))
                  (for _array_element (`/Game/Blueprints/Entities/AiEntity_BP.FootstepEntities` _asai_entity_bp)
                    (`/Engine/EditorBlueprintResources/StandardMacros.IsValid` _array_element
                      (:`Is Valid`
                        (set `/Game/Blueprints/Entities/FootprintEntity_BP.Host` _asai_entity_bp _array_element))))
                  (`self.SetVisuals&PhysicalEvent` _asai_entity_bp)
                  (`self.K2_DestroyActor`))))))))))

(fn `UserConstructionScript`
  (`parent.UserConstructionScript`))