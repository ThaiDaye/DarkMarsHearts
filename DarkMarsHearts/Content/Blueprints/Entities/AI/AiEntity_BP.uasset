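; AI entity base Blueprint that leaves footprints, can be grabbed off surfaces and can reattach on impact.
; Looping timers spawn footprint entities while moving, sample velocity and call a currently empty LeapEvent.
; GrabEvent enables box physics and opens a gate after a random delay, letting qualifying non-entity hits randomly stop simulation unless frozen, broken or chained.
; Impulse-based leap and line-of-sight logic remains disconnected.
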(event `LeaveFootprint`
  (bind _returnvalue (`self.K2_GetActorLocation`))
  ;[1 1 1] footprints
  (if (not (== (`self.MoveSpeed`) 0.0))
    (bind _outhit (`KismetSystemLibrary.SphereTraceSingleForObjects` _returnvalue _returnvalue 50.0 (`|MakeArray` "ObjectTypeQuery1" :!type "EObjectTypeQuery Enum")))
    (bind (_bblockinghit _binitialoverlap _time _distance _location _impactpoint) (`GameplayStatics.BreakHitResult` _outhit))
    (if _bblockinghit
      (`|SpawnActorFromClass` :`Class` "/Game/Blueprints/Entities/MarkingVariants/FootprintEntity_BP.FootprintEntity_BP_C" :`SpawnTransform` (`KismetMathLibrary.MakeTransform` _impactpoint (`self.K2_GetActorRotation`)) :`CollisionHandlingOverride` "Undefined" :`TransformScaleMethod` "OverrideRootScale" :`Host` self :`EntityIcon` null :`VisualMaterial` "/Game/Materials/PhysicalMaterial_Mat_Default.PhysicalMaterial_Mat_Default" :`Instigator` null))))

(event `VelocityCheck`
  (set `self.AiVelocity` (`KismetMathLibrary.VSize` (- (`self.K2_GetActorLocation`) (`self.LastPosDEBUG`))))
  (set `self.LastPosDEBUG` (`self.K2_GetActorLocation`)))

(event `self.ReceiveBeginPlay`
  (`parent.ReceiveBeginPlay`)
  (`KismetSystemLibrary.K2_SetTimerDelegate` (delegate `LeapEvent`) (`KismetMathLibrary.RandomFloatInRange` 6.0 12.0) true)
  (`KismetSystemLibrary.K2_SetTimerDelegate` (delegate `LeaveFootprint`) 3.0 true)
  (`KismetSystemLibrary.K2_SetTimerDelegate` (delegate `VelocityCheck`) 0.5 true)
  (`SceneComponent.K2_AttachToComponent` (`self.MainMesh`) (`self.SpringArm`) "None" "KeepRelative" "KeepRelative" "KeepRelative" true))

(event `self.ReceiveHit`
  (params (MyComp :type "PrimitiveComponent Object Reference") (Other :type "Actor Object Reference") (OtherComp :type "PrimitiveComponent Object Reference") (bSelfMoved :type Boolean) (HitLocation :type "Vector Structure") (HitNormal :type "Vector Structure") (NormalImpulse :type "Vector Structure") (Hit :type "HitResult Structure (by ref)"))
  (`parent.ReceiveHit` MyComp Other OtherComp bSelfMoved HitLocation HitNormal NormalImpulse Hit)
  (`/Engine/EditorBlueprintResources/StandardMacros.Gate` true :!label _label
    (:`Exit`
      (cast `/Game/Blueprints/Entities/Entity_BP` Other
        (:`CastFailed`
          (if (`self.IsFrozen`)
            _
            (elif (== (`self.Durability`) 0.0)
              _
              (elif (`KismetArrayLibrary.Array_IsValidIndex` (`self.ChainRef`))
                _
                (elif (not (> (`KismetMathLibrary.RandomFloatInRange` 0.0 1.0) 0.25))
                  (`PrimitiveComponent.SetSimulatePhysics` (`self.Box`) false))))))))))

(event `GrabEvent`
  (`PrimitiveComponent.SetSimulatePhysics` (`self.Box`) true)
  (set `self.LeapingDEBUG` true)
  (`KismetSystemLibrary.Delay` (`KismetMathLibrary.RandomFloatInRange` 0.0 1.0))
  (goto _label :!via `Open`))

(event `LeapEvent`
  ;[1 0 0] Comment
)

(fn `UserConstructionScript`
  (`parent.UserConstructionScript`))