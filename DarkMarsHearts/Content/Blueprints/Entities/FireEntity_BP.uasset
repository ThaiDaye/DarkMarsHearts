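; Fire entity that burns a Host entity, spreads, and clears the Host's OnFire flag when destroyed.
; On spawn, if not moving, it sphere-traces static world geometry to leave a scaled burn mark.
; A one-second timer randomly spreads fire and rolls against Host flammability to deal density-scaled burn damage and apply temperature-based wetness reduction.
; Without a valid Host, on a failed roll or at zero Host durability, the fire damages itself instead.
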(event `self.ReceiveDestroyed`
  (bind _host (`self.Host`))
  (`/Engine/EditorBlueprintResources/StandardMacros.IsValid` _host
    (:`Is Valid`
      (set `/Game/Blueprints/Entities/Entity_BP.OnFire` false _host))))

(event `self.ReceiveBeginPlay`
  (bind _returnvalue (`self.K2_GetActorLocation`))
  (bind _velocitylatetick (`self.VelocityLateTick`))
  (bind _returnvalue_2 (`KismetMathLibrary.VSize` (`self.GetVelocity`)))
  (`parent.ReceiveBeginPlay`)
  (`KismetSystemLibrary.K2_SetTimerDelegate` (delegate `FireTick`) 1.0 true)
  (`PrimitiveComponent.SetCollisionResponseToChannel` (`self.Box`) "ECC_Pawn" "ECR_Overlap")
  ;[1 1 1] burn mark
  (if (== (select `bool` (> _velocitylatetick _returnvalue_2) :`false` _velocitylatetick :`true` _returnvalue_2) 0.0)
    (bind _outhit (`KismetSystemLibrary.SphereTraceSingleForObjects` _returnvalue _returnvalue (`KismetMathLibrary.VSize` (* (`self.GetActorScale3D`) 50.0)) (`|MakeArray` "ObjectTypeQuery1" :!type "EObjectTypeQuery Enum")))
    (bind (_bblockinghit _binitialoverlap _time _distance _location _impactpoint) (`GameplayStatics.BreakHitResult` _outhit))
    (if _bblockinghit
      (`|SpawnActorFromClass` :`Class` "/Game/Blueprints/Entities/MarkingVariants/BurnMarkingEntity_BP.BurnMarkingEntity_BP_C" :`SpawnTransform` (`KismetMathLibrary.MakeTransform` _impactpoint (struct) (`KismetMathLibrary.Conv_DoubleToVector` (`KismetMathLibrary.VSize` (`self.GetActorScale3D`)))) :`CollisionHandlingOverride` "AlwaysSpawn" :`TransformScaleMethod` "OverrideRootScale" :`Host` null :`EntityIcon` null :`VisualMaterial` "/Game/Materials/PhysicalMaterial_Mat_Default.PhysicalMaterial_Mat_Default" :`Instigator` null))))

(event `FireTick`
  (bind _host (`self.Host`))
  (bind _returnvalue (* (`self.Temperature`) (`self.FireLethality`)))
  (if (<= (`KismetMathLibrary.RandomFloatInRange` 0.0 1.0) 0.1)
    (`KismetSystemLibrary.PrintString` "FIRE SPREAD" true true (struct :`R` 1.0 :`B` 0.029373 :`A` 1.0))
    (`self.SpreadFire`))
  (`/Engine/EditorBlueprintResources/StandardMacros.IsValid` _host
    (:`Is Valid`
      (if (< (`KismetMathLibrary.RandomFloatInRange` 0.0 1.0) (select `/Game/Blueprints/Flammability_Types` (`/Game/Blueprints/Entities/Entity_BP.Flammability` _host) :`NewEnumerator0` 0.8 :`NewEnumerator1` 0.5 :!type "Float (single-precision)"))
        (if (== (`/Game/Blueprints/Entities/Entity_BP.Durability` _host) 0.0)
          (`self.ReduceDurability` (* (`self.Temperature`) (`self.FireLethality`)) true true :!label _label)
          (else
            (`/Engine/EditorBlueprintResources/StandardMacros.IsValid` _host
              (:`Is Valid`
                (`self.ReduceDurability` _host (`KismetMathLibrary.FClamp` (+ _returnvalue (* (`KismetMathLibrary.FClamp` (- 1.5 (`/Game/Blueprints/Entities/Entity_BP.Density` _host))) _returnvalue)) 0.0 999999.0) true true false false (0.0 0.0 0.0))
                (`self.ApplyWetness` _host (`self.TempTo%age` (`self.Temperature`)) true "NewEnumerator0"))
              (:`Is Not Valid`
                (goto _label)))))
        (else
          (goto _label))))
    (:`Is Not Valid`
      (goto _label))))

(fn `UserConstructionScript`
  (`parent.UserConstructionScript`))