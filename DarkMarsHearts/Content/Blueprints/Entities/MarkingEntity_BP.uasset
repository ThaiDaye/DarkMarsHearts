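; MarkingEntity_BP is a surface decal entity, a marking that gradually fades and then removes itself.
; On BeginPlay a small sphere trace against WorldStatic orients the decal to the hit normal, or destroys the actor when nothing blocks.
; It copies Temperature from a valid Host.
; A looping timer applies random durability loss, drives the dynamic material's opacity from remaining durability and destroys the actor at zero.
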(event `self.ReceiveBeginPlay`
  (bind _host (`self.Host`))
  (bind _returnvalue (`SceneComponent.K2_GetComponentLocation` (`self.Box`)))
  (`parent.ReceiveBeginPlay`)
  (bind _outhit (`KismetSystemLibrary.SphereTraceSingleForObjects` _returnvalue _returnvalue 25.0 (`|MakeArray` "ObjectTypeQuery1" :!type "EObjectTypeQuery Enum")))
  (bind (_bblockinghit _binitialoverlap _time _distance _location _impactpoint _normal) (`GameplayStatics.BreakHitResult` _outhit))
  (if _bblockinghit
    (bind (_returnvalue_roll _returnvalue_pitch _returnvalue_yaw) (`KismetMathLibrary.BreakRotator` (`KismetMathLibrary.Conv_VectorToRotator` _normal)))
    (`SceneComponent.K2_SetWorldRotation` (`self.Decal`) (`KismetMathLibrary.MakeRotator` _returnvalue_roll _returnvalue_pitch _returnvalue_yaw) false false)
    (`KismetSystemLibrary.K2_SetTimerDelegate` (delegate `DecayTick`) 1.0 true)
    (bind _returnvalue_2 (`DecalComponent.CreateDynamicMaterialInstance` (`self.Decal`)))
    (`/Engine/EditorBlueprintResources/StandardMacros.IsValid` _host
      (:`Is Valid`
        (set `self.Temperature` (`/Game/Blueprints/Entities/Entity_BP.Temperature` _host))))
    (else
      (`self.K2_DestroyActor`))))

(event `DecayTick`
  (`self.ReduceDurability` (`KismetMathLibrary.RandomFloatInRange` (`self.DecayMin`) (`self.DecayMax`)))
  (`MaterialInstanceDynamic.SetScalarParameterValue` (stale `self.ReceiveBeginPlay` _returnvalue_2) "opacity_max" (/ (`self.Durability`) (`self.MaxDurability`)))
  (if (== (`self.Durability`) 0.0)
    (`self.K2_DestroyActor`)))

(fn `UserConstructionScript`
  (`parent.UserConstructionScript`))