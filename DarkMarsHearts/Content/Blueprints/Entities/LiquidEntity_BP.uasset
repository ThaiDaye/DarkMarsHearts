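; Liquid entity that flies as a mesh blob and becomes a decal puddle on hitting the environment, with material set by liquid type.
; Non-metal, non-Martian blobs are consumed on hitting reactive entities, cleaning marks or applying wetness.
; Overlaps merge same-type liquids and let puddles transfer liquid to entities.
; Durability acts as volume, driving scale, mass and wetness, while a looping timer feeds temperature state to the decal material.
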(event `SetDecalVisualParameters`
  (bind _decalref (`self.DecalRef`))
  (`MeshComponent.SetScalarParameterValueOnMaterials` _decalref "MeltingPoint" (`self.TemperaturePerSecMelt`))
  (`MeshComponent.SetScalarParameterValueOnMaterials` _decalref "FreezingPoint" (`self.TemperaturePerSecFreeze`))
  (`MeshComponent.SetScalarParameterValueOnMaterials` _decalref "Frozen" (`self.IsFrozenPerSec`))
  (`MeshComponent.SetScalarParameterValueOnMaterials` _decalref "Wetness_Oil" (select `bool` (`|EnumEquality` (`self.WetnessType`) "NewEnumerator2") :`true` 1.0 :!type "Float (single-precision)"))
  (`DecalComponent.SetDecalMaterial` (`self.Decal`) (`PrimitiveComponent.GetMaterial` (`self.DecalRef`) 0))
  (set `self.Mass` (* 10.0 (`KismetMathLibrary.Lerp` 1.0 10.0 (/ (`self.Durability`) (`self.MaxDurability`)))))
  (`self.WeightEvent`))

(event `self.ReceiveHit`
  (params (MyComp :type "PrimitiveComponent Object Reference") (Other :type "Actor Object Reference") (OtherComp :type "PrimitiveComponent Object Reference") (bSelfMoved :type Boolean) (HitLocation :type "Vector Structure") (HitNormal :type "Vector Structure") (NormalImpulse :type "Vector Structure") (Hit :type "HitResult Structure (by ref)"))
  (`parent.ReceiveHit` MyComp Other OtherComp bSelfMoved HitLocation HitNormal NormalImpulse Hit)
  (if (not (select `/Game/Blueprints/P_Liquid_Types` (`self.LiquidType`) :`NewEnumerator3` true :`NewEnumerator4` true))
    (bind _asentity_bp (cast `/Game/Blueprints/Entities/Entity_BP` Other)
      (:`then`
        (bind _asmarking_entity_bp (cast `/Game/Blueprints/Entities/MarkingEntity_BP` _asentity_bp)
          (:`then`
            (if (not (`|EnumEquality` (`/Game/Blueprints/Entities/Entity_BP.HydroReaction` _asmarking_entity_bp) "NewEnumerator0"))
              ;[1 1 1] cleaing up marks
              (`self.ReduceDurability` _asmarking_entity_bp (`self.Durability`) false true false false (0.0 0.0 0.0))
              (`self.K2_DestroyActor`)))
          (:`CastFailed`
            (cast `/Game/Blueprints/Entities/LiquidEntity_BP` _asentity_bp
              (:`CastFailed`
                (cast `/Game/Blueprints/Entities/GasEntity_BP` _asentity_bp
                  (:`CastFailed`
                    (if (`self.Connected`)
                      _
                      (elif (not (`|EnumEquality` (`/Game/Blueprints/Entities/Entity_BP.HydroReaction` _asentity_bp) "NewEnumerator0"))
                        (`KismetSystemLibrary.PrintString` "LIQUID HIT ENTITY" true true (struct :`G` 1.0 :`B` 0.975202 :`A` 1.0))
                        (`self.ApplyWetness` _asentity_bp (* (`self.Durability`) 0.005) false (`self.LiquidType`))
                        (`self.K2_DestroyActor`))))))))))
      (:`CastFailed`
        (cast `/Game/Blueprints/Entities/PlayerEntity_BP` Other
          (:`CastFailed`
            (`KismetSystemLibrary.PrintString` "LIQUID HIT ENVIRONMENT" true true (struct :`G` 1.0 :`B` 0.975202 :`A` 1.0))
            (set `self.Connected` true)
            (`self.ConnectedEvent`)
            (`self.SetLiquidVisual`)
            (`self.SetDecalFacing`)))))))

(event `self.ReceiveBeginPlay`
  (`parent.ReceiveBeginPlay`)
  (`self.SetLiquidVisual`)
  (`KismetSystemLibrary.K2_SetTimerDelegate` (delegate `SetDecalVisualParameters`) 0.005 true)
  (if (select `/Game/Blueprints/P_Liquid_Types` (`self.LiquidType`) :`NewEnumerator3` true :`NewEnumerator4` true)
    (`SceneComponent.SetRelativeScale3D` (`self.Box1`) (0.75 0.5 0.5))
    (`KismetSystemLibrary.Delay` 1.0))
  (set `self.LiquidImpactRef` true))

(event `self.Box1.OnComponentBeginOverlap`
  (params (OverlappedComponent :type "PrimitiveComponent Object Reference") (OtherActor :type "Actor Object Reference") (OtherComp :type "PrimitiveComponent Object Reference") (OtherBodyIndex :type Integer) (bFromSweep :type Boolean) (SweepResult :type "HitResult Structure (by ref)"))
  (bind _durability (`self.Durability`))
  (cast `/Game/Blueprints/Entities/TemperatureEntity_BP` OtherActor
    (:`CastFailed`
      (if (`self.LiquidImpactRef`)
        (if (not (== OtherActor self))
          (bind _asliquid_entity_bp (cast `/Game/Blueprints/Entities/LiquidEntity_BP` OtherActor)
            (:`then`
              (`/Engine/EditorBlueprintResources/StandardMacros.IsValid` _asliquid_entity_bp
                (:`Is Valid`
                  (if (`/Game/Blueprints/Entities/LiquidEntity_BP.LiquidImpactRef` _asliquid_entity_bp)
                    (if (`|EnumEquality` (`/Game/Blueprints/Entities/LiquidEntity_BP.LiquidType` _asliquid_entity_bp) (`self.LiquidType`))
                      (if (`/Game/Blueprints/Entities/Entity_BP.Connected` _asliquid_entity_bp)
                        (if (>= (`/Game/Blueprints/Entities/Entity_BP.Durability` _asliquid_entity_bp) _durability) :!label _label
                          (`self.ReduceDurability` _asliquid_entity_bp (* _durability -1.0) false true false false (0.0 0.0 0.0))
                          (`self.SetLiquidVisual` _asliquid_entity_bp)
                          (`KismetSystemLibrary.PrintString` "LIQUID COMBINED" true true (struct :`G` 1.0 :`B` 0.973628 :`A` 1.0))
                          (`self.K2_DestroyActor`))
                        (elif (not (`self.Connected`))
                          (goto _label))))))))
            (:`CastFailed`
              ;[1 1 1] wet from puddle
              (if (`self.Connected`)
                (cast `/Game/Blueprints/Entities/GasEntity_BP` OtherActor
                  (:`CastFailed`
                    (bind _asentity_bp (cast `/Game/Blueprints/Entities/Entity_BP` OtherActor))
                    (`/Engine/EditorBlueprintResources/StandardMacros.IsValid` _asentity_bp
                      (:`Is Valid`
                        (bind _hydroreaction (`/Game/Blueprints/Entities/Entity_BP.HydroReaction` _asentity_bp))
                        (if (`|EnumEquality` _hydroreaction "NewEnumerator0")
                          _
                          (elif (>= (`/Game/Blueprints/Entities/Entity_BP.Wetness` _asentity_bp) 1.0)
                            (if (`|EnumEquality` _hydroreaction "NewEnumerator2")
                              (`self.TransferLiquids` _asentity_bp 20.0 :!label _label_2)
                              (`KismetSystemLibrary.PrintString` "WET FROM LIQUID PUDDLE" true true (struct :`G` 0.362928 :`B` 1.0 :`A` 1.0)))
                            (else
                              (goto _label_2))))))))))))))))

(event `SetLiquidVisual`
  (bind _box1 (`self.Box1`))
  (bind _mainmesh (`self.MainMesh`))
  (bind _decal (`self.Decal`))
  (bind _box (`self.Box`))
  (bind _returnvalue (select `/Game/Blueprints/P_Liquid_Types` (`self.LiquidType`) :`NewEnumerator0` "/Game/Materials/LiquidMaterial_Mat_Default.LiquidMaterial_Mat_Default" :`NewEnumerator1` "/Game/Materials/LiquidMaterial_Mat_Default.LiquidMaterial_Mat_Default" :`NewEnumerator2` "/Game/Materials/LiquidMaterial_Mat_Default.LiquidMaterial_Mat_Default" :`NewEnumerator3` "/Game/Materials/LiquidMaterial_Mat_Default.LiquidMaterial_Mat_Default" :`NewEnumerator4` "/Game/Materials/LiquidMaterial_Mat_Martian.LiquidMaterial_Mat_Martian" :!type "MaterialInstance Object Reference"))
  (bind _returnvalue_2 (`KismetMathLibrary.Lerp` 0.5 4.0 (/ (`self.Durability`) (`self.MaxDurability`))))
  ;[1 1 1] set visual
  (`PrimitiveComponent.SetMaterial` (`self.DecalRef`) 0 _returnvalue)
  (`DecalComponent.SetDecalMaterial` (`self.Decal`) _returnvalue)
  (bind _output_get (set `self.VisualMaterial` (select `/Game/Blueprints/P_Liquid_Types` (`self.LiquidType`) :`NewEnumerator0` "/Game/Materials/TransparentMaterial_Mat_Default.TransparentMaterial_Mat_Default" :`NewEnumerator1` "/Game/Materials/TransparentMaterial_Mat_Default.TransparentMaterial_Mat_Default" :`NewEnumerator2` "/Game/Materials/TransparentMaterial_Mat_Default.TransparentMaterial_Mat_Default" :`NewEnumerator3` "/Game/Materials/PhysicalMaterial_Mat_LiquidMetal.PhysicalMaterial_Mat_LiquidMetal" :`NewEnumerator4` "/Game/Materials/PhysicalMaterial_Mat_Rust_Liquid.PhysicalMaterial_Mat_Rust_Liquid" :!type "MaterialInstance Object Reference")))
  (`PrimitiveComponent.SetMaterial` (`self.MainMesh`) 0 _output_get)
  (`self.SetActorScale3D` (`KismetMathLibrary.MakeVector` _returnvalue_2 _returnvalue_2 _returnvalue_2))
  (`BoxComponent.SetBoxExtent` _box1 (`BoxComponent.BoxExtent` _box1) true)
  (set `self.WetnessType` (`self.LiquidType`))
  (if (and (`KismetSystemLibrary.IsValid` _box) (`KismetSystemLibrary.IsValid` _mainmesh) (`KismetSystemLibrary.IsValid` _decal))
    (if (`self.Connected`)
      (`SceneComponent.SetVisibility` _mainmesh false false)
      (`SceneComponent.SetVisibility` _decal true false)
      (`PrimitiveComponent.SetCollisionResponseToChannel` _box "ECC_Vehicle" "ECR_Ignore")
      (`PrimitiveComponent.SetCollisionResponseToChannel` _box "ECC_Pawn" "ECR_Overlap")
      (else
        (`SceneComponent.SetVisibility` _mainmesh true false)
        (`SceneComponent.SetVisibility` _decal false false)
        (`PrimitiveComponent.SetCollisionResponseToChannel` _box "ECC_Vehicle" "ECR_Block")
        (`PrimitiveComponent.SetCollisionResponseToChannel` _box "ECC_Pawn" "ECR_Block")))))

(event `SetDecalFacing`
  (bind _decal (`self.Decal`))
  (bind _returnvalue (`SceneComponent.K2_GetComponentLocation` (`self.Box`)))
  (bind (_relativerotation_roll _relativerotation_pitch _relativerotation_yaw) (`KismetMathLibrary.BreakRotator` (`SceneComponent.RelativeRotation` _decal)))
  ;[1 1 1] set visual
  (bind _outhit (`KismetSystemLibrary.SphereTraceSingleForObjects` _returnvalue _returnvalue 30.0 (`|MakeArray` "ObjectTypeQuery1" "ObjectTypeQuery3" :!type "EObjectTypeQuery Enum")))
  (`/Engine/EditorBlueprintResources/StandardMacros.IsValid` _decal
    (:`Is Valid`
      (`SceneComponent.K2_SetWorldRotation` _decal (`KismetMathLibrary.Conv_VectorToRotator` (`.Normal` (`GameplayStatics.BreakHitResult` _outhit))) false false)
      (`/Engine/EditorBlueprintResources/StandardMacros.IsValid` _decal
        (:`Is Valid`
          (`SceneComponent.K2_SetRelativeRotation` _decal (`KismetMathLibrary.MakeRotator` (`KismetMathLibrary.RandomFloatInRange` -180.0 180.0) _relativerotation_pitch _relativerotation_yaw) false false))))))

(fn `UserConstructionScript`
  (`parent.UserConstructionScript`)
  (`self.SetLiquidVisual`))