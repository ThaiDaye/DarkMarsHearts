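; Test actor for an AI tendril that hunts the player, where one class serves as head, body segment and base.
; The head spawns a chain of followers, then steers toward the player on looping timers with random wobble, deflecting off blocking hits.
; When a connected base gets pulled, the chain freezes and the head retracts along it, destroying segments, then respawns a new tendril after a random delay.
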(event `self.ReceiveBeginPlay`
  (bind _segmentcount (`self.SegmentCount`))
  (bind _f (`self.f`))
  (bind _lastsegref (`self.LastSegRef`))
  (bind _returnvalue (select `bool` (`KismetSystemLibrary.IsValid` _lastsegref) :`false` self :`true` _lastsegref :!type "/Game/Blueprints/Entities/WIP/AITendrilEntity_TestBP Object Reference"))
  (bind (_returnvalue_location _returnvalue_rotation _returnvalue_scale) (`KismetMathLibrary.BreakTransform` (`self.GetTransform` _returnvalue)))
  (if (`self.Head`)
    (if (`self.AutoGen`)
      (for _index (range 1 (+ _segmentcount 1))
        (bind _returnvalue_2 (`|SpawnActorFromClass` "AITendrilEntity_TestBP_C" (`KismetMathLibrary.MakeTransform` _returnvalue_location _returnvalue_rotation _returnvalue_scale) "AlwaysSpawn" "OverrideRootScale" null false (== _index _segmentcount) (`self.Connected`) _returnvalue (`self.Speed`) (`self.BodyRadius`) (`self.TurnTightness`) true 16 self null))
        (`KismetArrayLibrary.Array_Add` (`self.HeadChildren`) _returnvalue_2)
        (set `self.LastSegRef` _returnvalue_2)))
    (`PrimitiveComponent.SetMaterial` _f 0 "/Game/Materials/PhysicalMaterial_Mat_Rust.PhysicalMaterial_Mat_Rust")
    (for _array_element (`self.HeadChildren`)
      (`/Engine/EditorBlueprintResources/StandardMacros.IsValid` _array_element
        (:`Is Valid`
          (set `/Game/Blueprints/Entities/WIP/AITendrilEntity_TestBP.Speed` (`self.Speed`) _array_element))))
    (else
      (`PrimitiveComponent.SetCollisionObjectType` _f "ECC_WorldDynamic")))
  (`KismetSystemLibrary.K2_SetTimerDelegate` (delegate `Move`) 0.05 true)
  (`KismetSystemLibrary.K2_SetTimerDelegate` (delegate `Rotate`) 0.25 true)
  (`KismetSystemLibrary.K2_SetTimerDelegate` (delegate `ReverseToSeg`) 0.3 true))

(event `ReverseToSeg`
  (bind _headchildren (`self.HeadChildren`))
  (bind _output (`|GetArrayItem` _headchildren))
  (bind _returnvalue (`self.K2_GetActorLocation` _output))
  ;[1 1 1] return
  (if (`self.Reversing`)
    (if (`self.Head`)
      (bind (_direction _newtrack_0) (`Timeline|Timeline_0` :!via `PlayFromStart`)
        (:`Update`
          (`/Engine/EditorBlueprintResources/StandardMacros.IsValid` _output
            (:`Is Valid`
              (`self.K2_SetActorLocation` (`KismetMathLibrary.VLerp` (`self.K2_GetActorLocation`) _returnvalue _newtrack_0))
              (`self.K2_SetActorRotation` (`KismetMathLibrary.RLerp` (`self.K2_GetActorRotation`) (`self.K2_GetActorRotation` _output) _newtrack_0 true)))))
        (:`Finished`
          (`/Engine/EditorBlueprintResources/StandardMacros.IsValid` _output
            (:`Is Valid`
              (`self.K2_SetActorLocation` _returnvalue)
              (`self.K2_DestroyActor` _output)
              (`KismetArrayLibrary.Array_Remove` _headchildren))
            (:`Is Not Valid`
              (if (== (`KismetArrayLibrary.Array_Length` _headchildren) 0)
                (`KismetSystemLibrary.Delay` (`KismetMathLibrary.RandomFloatInRange` 0.0 2.0))
                (`|SpawnActorFromClass` "AITendrilEntity_TestBP_C" (`self.GetTransform`) "AlwaysSpawn" "OverrideRootScale" null true false (`self.Connected`) null (`self.Speed`) (`self.BodyRadius`) (`self.TurnTightness`) (`self.AutoGen`) (`self.SegmentCount`) null null)
                (`self.K2_DestroyActor`)))))))))

(event `Move`
  (bind _speed (`self.Speed`))
  (bind _f (`self.f`))
  (bind _target (`self.target`))
  (bind _f_2 (`self.f`))
  (bind _returnvalue (`self.GetDistanceTo` _target))
  (if (`self.Reversing`)
    _
    (elif (`self.Head`)
      (bind _sweephitresult (`SceneComponent.K2_AddWorldOffset` _f (* (`SceneComponent.GetForwardVector` (`self.Arrow`)) _speed) true false))
      (bind (_bblockinghit _binitialoverlap _time _distance _location _impactpoint _normal _impactnormal) (`GameplayStatics.BreakHitResult` _sweephitresult))
      (if _bblockinghit
        (`SceneComponent.K2_SetWorldRotation` _f_2 (`KismetMathLibrary.RLerp` (`KismetMathLibrary.Conv_VectorToRotator` _impactnormal) (`SceneComponent.K2_GetComponentRotation` _f_2) 0.5 true) false false))
      (else
        (`SceneComponent.K2_AddWorldOffset` _f (select `bool` (< _returnvalue (`self.BodyRadius`)) :`false` (* (`KismetMathLibrary.Conv_RotatorToVector` (`KismetMathLibrary.FindLookAtRotation` (`self.K2_GetActorLocation`) (`self.K2_GetActorLocation` _target))) (* _speed 1.25))) false false)
        (if (`self.Base`)
          (if (> _returnvalue (* (`self.BodyRadius`) 0.5))
            (if (`self.Connected`)
              (`KismetSystemLibrary.PrintString` "BASE MOVED" true true (struct :`R` 1.0 :`G` 0.01 :`A` 1.0))
              (set `self.Reversing` true)
              (`self.HeadReverse` (`self.headRef`)))))))))

(event `Rotate`
  (bind _f (`self.f`))
  (bind _speed (`self.Speed`))
  (bind _returnvalue (* _speed -1.0))
  (if (`self.Reversing`)
    _
    (elif (`self.Head`)
      (`SceneComponent.K2_SetWorldRotation` _f (`KismetMathLibrary.RLerp` (`SceneComponent.K2_GetComponentRotation` _f) (`KismetMathLibrary.FindLookAtRotation` (`self.K2_GetActorLocation`) (`self.K2_GetActorLocation` (`GameplayStatics.GetPlayerCharacter` 0))) (`self.TurnTightness`) true) false false)
      (`SceneComponent.K2_AddLocalRotation` _f (`KismetMathLibrary.MakeRotator` (`KismetMathLibrary.RandomFloatInRange` _returnvalue _speed) (`KismetMathLibrary.RandomFloatInRange` _returnvalue _speed)) false false)
      (else
        (`SceneComponent.K2_SetWorldRotation` _f (`KismetMathLibrary.FindLookAtRotation` (`self.K2_GetActorLocation`) (`self.K2_GetActorLocation` (`self.target`))) false false)))))

(fn `HeadReverse`
  (for _array_element (`self.HeadChildren`)
    (`/Engine/EditorBlueprintResources/StandardMacros.IsValid` _array_element
      (:`Is Valid`
        (set `/Game/Blueprints/Entities/WIP/AITendrilEntity_TestBP.Reversing` true _array_element))))
  (set `self.Reversing` true))

(fn `UserConstructionScript`
  (bind _target (`self.target`))
  (`/Engine/EditorBlueprintResources/StandardMacros.IsValid` _target
    (:`Is Valid`
      (set `self.Speed` (`/Game/Blueprints/Entities/WIP/AITendrilEntity_TestBP.Speed` _target)))))