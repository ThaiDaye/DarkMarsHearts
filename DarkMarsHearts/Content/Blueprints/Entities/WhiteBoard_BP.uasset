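; Interactable whiteboard the player draws and erases on, with four marker colours, an eraser and a clear button.
; While the board is held in interaction, a Gate and Delay loop sphere-traces from the first-person camera and moves a cursor marker.
; Ink dots are instances in per-colour instanced static meshes, removed on erasing.
; Parallel arrays record each dot's location, normal, scale and colour for LoadBoard to rebuild, though ClearBoard clears only instances.
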(event `self.Interact`
  (params (SubObject :type "ActorComponent Object Reference") (HitLocation :type "Vector Structure") (HitNormal :type "Vector Structure") (PlayerInteract :type Boolean))
  (bind _array (`|MakeArray` "ObjectTypeQuery1" :!type "EObjectTypeQuery Enum"))
  (bind _currentcolour (`self.CurrentColour`))
  (bind _currentcolour_2 (`self.CurrentColour`))
  (bind _firstpersoncamera (`/Game/Blueprints/Entities/PlayerEntity_BP.FirstPersonCamera` (`self.PlayerRef`)))
  (bind _returnvalue (`SceneComponent.K2_GetComponentLocation` _firstpersoncamera))
  (bind _returnvalue_2 (+ _returnvalue (* (`SceneComponent.GetForwardVector` _firstpersoncamera) 100000.0)))
  (`parent.Interact` SubObject HitLocation HitNormal false)
  (if (== SubObject (`self.MainMesh`))
    (`SceneComponent.SetVisibility` (`self.Cursor_marker`) true true)
    (`PrimitiveComponent.SetMaterial` (`self.Cursor_Marker_Mesh`) 0 (select `bool` (== _currentcolour -1) :`false` (select `int` _currentcolour :`0` "/Game/Materials/Ink_mat.Ink_mat" :`1` "/Game/Materials/Ink_mat1.Ink_mat1" :`2` "/Game/Materials/Ink_mat2.Ink_mat2" :`3` "/Game/Materials/Ink_mat3.Ink_mat3" :!type "MaterialInterface Object Reference") :`true` "/Game/Materials/PhysicalMaterial_Mat_White.PhysicalMaterial_Mat_White"))
    (`|ExecutionSequence`
      (:`then_0`
        (goto _label :!via `Open`))
      (:`then_1`
        (`/Engine/EditorBlueprintResources/StandardMacros.Gate` true :!label _label
          (:`Exit`
            (`|ExecutionSequence`
              (:`then_0`
                (if (== (`self.CurrentColour`) -1)
                  (bind _outhits (`KismetSystemLibrary.SphereTraceMultiForObjects` :`Start` _returnvalue :`End` _returnvalue_2 :`Radius` 10.0 :`ObjectTypes` _array :`bIgnoreSelf` false))
                  (for _array_element _outhits
                    (bind (_bblockinghit _binitialoverlap _time _distance _location _impactpoint _normal _impactnormal _physmat _hitactor _hitcomponent _hitbonename _hititem) (`GameplayStatics.BreakHitResult` _array_element))
                    (bind _asinstanced_static_mesh_component (cast `InstancedStaticMeshComponent` _hitcomponent))
                    (`InstancedStaticMeshComponent.RemoveInstance` _asinstanced_static_mesh_component _hititem)
                    (`KismetArrayLibrary.Array_Remove` (`self.InkScale`) _hititem)
                    (`KismetArrayLibrary.Array_Remove` (`self.InkLocations`) _hititem)
                    (`KismetArrayLibrary.Array_Remove` (`self.InkNormals`) _hititem)
                    (`KismetArrayLibrary.Array_Remove` (`self.InkColour`) _hititem)
                    (`SceneComponent.K2_SetWorldLocation` (`self.Cursor_marker`) _impactpoint false false))
                  (else
                    (bind _outhit (`KismetSystemLibrary.SphereTraceSingleForObjects` :`Start` _returnvalue :`End` _returnvalue_2 :`Radius` 2.0 :`ObjectTypes` _array :`bIgnoreSelf` false))
                    (if (== _currentcolour_2 -1)
                      (bind (_bblockinghit_2 _binitialoverlap_2 _time_2 _distance_2 _location_2 _impactpoint_2 _normal_2 _impactnormal_2 _physmat_2 _hitactor_2 _hitcomponent_2 _hitbonename_2 _hititem_2) (`GameplayStatics.BreakHitResult` _outhit))
                      (bind _asinstanced_static_mesh_component_2 (cast `InstancedStaticMeshComponent` _hitcomponent_2 :!label _label_2))
                      (`InstancedStaticMeshComponent.RemoveInstance` _asinstanced_static_mesh_component_2 _hititem_2)
                      (`KismetArrayLibrary.Array_Remove` (`self.InkScale`) _hititem_2)
                      (`KismetArrayLibrary.Array_Remove` (`self.InkLocations`) _hititem_2)
                      (`KismetArrayLibrary.Array_Remove` (`self.InkNormals`) _hititem_2)
                      (`KismetArrayLibrary.Array_Remove` (`self.InkColour`) _hititem_2)
                      (`SceneComponent.K2_SetWorldLocation` (`self.Cursor_marker`) _impactpoint_2 false false :!label _label_3)
                      (elif (== (select `int` _currentcolour_2 :`0` (`self.Ink_01`) :`1` (`self.Ink_02`) :`2` (`self.Ink_03`) :`3` (`self.Ink_04`) :!type "Object Object Reference") _hitcomponent_2)
                        _
                        (elif (== _hitcomponent_2 (`self.MainMesh`))
                          (`self.AddInk` _impactpoint_2 _normal_2 0.05)
                          (goto _label_3)
                          (else
                            (goto _label_2))))))))
              (:`then_1`
                (`KismetSystemLibrary.Delay` 0.001)
                (goto _label)))))))
    (elif (== SubObject (`self.Clear`))
      (`self.ClearBoard`)
      (else
        (set `self.CurrentColour` (select `bool` (== SubObject (`self.Eraser`)) :`false` (select `bool` (== SubObject (`self.Marker_04`)) :`false` (select `bool` (== SubObject (`self.Marker_03`)) :`false` (select `bool` (== SubObject (`self.Marker_02`)) :`false` (select `bool` (== SubObject (`self.Marker_01`))) :`true` 1) :`true` 2) :`true` 3) :`true` -1))))))

(event `self.InteractEnd`
  (params (`Player Interact` :type Boolean))
  (`parent.InteractEnd` false)
  (`SceneComponent.SetVisibility` (`self.Cursor_marker`) false true)
  (goto _label :!via `Close`))

(fn `AddInk`
  (params (Location :type "Vector Structure") (Normal :type "Vector Structure") (Scale :type "Float (double-precision)"))
  (bind _currentcolour (`self.CurrentColour`))
  (bind _returnvalue (`KismetMathLibrary.MakeTransform` Location (`KismetMathLibrary.Conv_VectorToRotator` Normal) (`KismetMathLibrary.MakeVector` (* Scale 0.05) Scale Scale)))
  (switch `int` _currentcolour
    (:`0`
      (`InstancedStaticMeshComponent.AddInstanceWorldSpace` (`self.Ink_01`) _returnvalue))
    (:`1`
      (`InstancedStaticMeshComponent.AddInstanceWorldSpace` (`self.Ink_02`) _returnvalue))
    (:`2`
      (`InstancedStaticMeshComponent.AddInstanceWorldSpace` (`self.Ink_03`) _returnvalue))
    (:`3`
      (`InstancedStaticMeshComponent.AddInstanceWorldSpace` (`self.Ink_04`) _returnvalue)))
  (`KismetArrayLibrary.Array_Add` (`self.InkLocations`) Location)
  (`KismetArrayLibrary.Array_Add` (`self.InkNormals`) Normal)
  (`KismetArrayLibrary.Array_Add` (`self.InkScale`) Scale)
  (`KismetArrayLibrary.Array_Add` (`self.InkColour`) _currentcolour))

(fn `ClearBoard`
  (`InstancedStaticMeshComponent.ClearInstances` (`self.Ink_01`))
  (`InstancedStaticMeshComponent.ClearInstances` (`self.Ink_02`))
  (`InstancedStaticMeshComponent.ClearInstances` (`self.Ink_03`))
  (`InstancedStaticMeshComponent.ClearInstances` (`self.Ink_04`)))

(fn `LoadBoard`
  (for (_array_element _array_index) (`self.InkLocations`)
    (switch `int` (`|GetArrayItem` (`self.InkColour`) _array_index)
      (:`0`
        (bind _output (`|GetArrayItem` (`self.InkScale`) _array_index))
        (bind _returnvalue (`KismetMathLibrary.MakeTransform` _array_element (`KismetMathLibrary.Conv_VectorToRotator` (`|GetArrayItem` (`self.InkNormals`) _array_index)) (`KismetMathLibrary.MakeVector` _output _output _output)))
        (`InstancedStaticMeshComponent.AddInstanceWorldSpace` (`self.Ink_01`) _returnvalue))
      (:`1`
        (`InstancedStaticMeshComponent.AddInstanceWorldSpace` (`self.Ink_02`) _returnvalue))
      (:`2`
        (`InstancedStaticMeshComponent.AddInstanceWorldSpace` (`self.Ink_03`) _returnvalue))
      (:`3`
        (`InstancedStaticMeshComponent.AddInstanceWorldSpace` (`self.Ink_04`) _returnvalue)))))

(fn `UserConstructionScript`)