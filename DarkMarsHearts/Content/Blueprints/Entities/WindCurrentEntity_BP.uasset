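; Wind current volume that pushes, pulls or removes gravity from physics-simulating Entity_BP actors inside its box, ignoring temperature entities.
; Push follows the arrow and Pull draws toward it, applying weight-reduced velocity impulses to unconnected entities once or on a looping timer.
; ZeroG disables gravity via overlap events and polling, restoring it on exit or deactivation.
; Niagara effects take their parameters from box size, type and intensity, with visibility following Active.
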(event `ApplyWindPressure`
  (bind _intensity (`self.Intensity`))
  (if (`self.Active`)
    (if (not (or (== (`self.Intensity`) 0.0) (select `/Game/Blueprints/WindCurrent_Types` (`self.WindCurrentType`) :`NewEnumerator0` true :`NewEnumerator3` true)))
      (for _array_element (`PrimitiveComponent.GetOverlappingActors` (`self.Box`) "/Game/Blueprints/Entities/Entity_BP.Entity_BP_C")
        (bind _asentity_bp (cast `/Game/Blueprints/Entities/Entity_BP` _array_element))
        (cast `/Game/Blueprints/Entities/TemperatureEntity_BP` _array_element
          (:`CastFailed`
            (if (not (`/Game/Blueprints/Entities/Entity_BP.Connected` _asentity_bp))
              (bind _box (`/Game/Blueprints/Entities/Entity_BP.Box` _asentity_bp))
              (if (`SceneComponent.IsSimulatingPhysics` _box "None")
                (bind _returnvalue (* (select `/Game/Blueprints/WindCurrent_Types` (`self.WindCurrentType`) :`NewEnumerator1` (`SceneComponent.GetForwardVector` (`self.Arrow`)) :`NewEnumerator2` (`KismetMathLibrary.Conv_RotatorToVector` (`KismetMathLibrary.FindLookAtRotation` (`self.K2_GetActorLocation` _asentity_bp) (`SceneComponent.K2_GetComponentLocation` (`self.Arrow`))))) _intensity))
                (`PrimitiveComponent.AddImpulse` _box (- _returnvalue (* _returnvalue (`KismetMathLibrary.FClamp` (/ (`/Game/Blueprints/Entities/Entity_BP.Weight` _asentity_bp) (* _intensity 0.05))))) "None" true)))))))))

(event `self.ReceiveBeginPlay`
  (bind _niagara (`self.Niagara`))
  (bind _niagara_2 (`self.Niagara`))
  (bind _windcurrenttype (`self.WindCurrentType`))
  (bind _intensity (`self.Intensity`))
  (bind _returnvalue (`KismetMathLibrary.VSize` (`BoxComponent.BoxExtent` (`self.Box`))))
  (`parent.ReceiveBeginPlay`)
  (`KismetSystemLibrary.K2_SetTimerDelegate` (delegate `SetGravityTick`) 0.1 true)
  (`SceneComponent.SetVisibility` (`self.Arrow`) (select `/Game/Blueprints/WindCurrent_Types` (`self.WindCurrentType`) :`NewEnumerator1` true :`NewEnumerator2` true) false)
  (`NiagaraComponent.SetNiagaraVariableFloat` _niagara "User.GasRadius" _returnvalue)
  (`NiagaraComponent.SetNiagaraVariableFloat` _niagara "User.PullRadius" (* _returnvalue 2.5))
  (`NiagaraComponent.SetNiagaraVariableInt` _niagara_2 "User.Spawn Count" (`KismetMathLibrary.FTrunc` (* _returnvalue 0.05)))
  (`NiagaraComponent.SetNiagaraVariableVec3` _niagara_2 "User.GravityDirection" (* (select `/Game/Blueprints/WindCurrent_Types` _windcurrenttype :`NewEnumerator1` (`KismetMathLibrary.Conv_RotatorToVector` (`SceneComponent.K2_GetComponentRotation` (`self.Arrow`)))) (* _intensity 2.0)))
  (`NiagaraComponent.SetNiagaraVariableVec3` _niagara_2 "User.AttractPos" (`SceneComponent.K2_GetComponentLocation` (`self.Arrow`)))
  (`NiagaraComponent.SetNiagaraVariableFloat` _niagara_2 "User.AttractStrength" (select `/Game/Blueprints/WindCurrent_Types` _windcurrenttype :`NewEnumerator2` (* _intensity 0.1)))
  (`KismetSystemLibrary.K2_SetTimerDelegate` (delegate `SetActiveVisuals`) 0.1 true)
  (if (`self.SingleFire`)
    (`self.ApplyWindPressure`)
    (else
      (`self.ApplyWindPressure`)
      (`KismetSystemLibrary.K2_SetTimerDelegate` (delegate `ApplyWindPressure`) 0.1 true))))

(event `SetGravityTick`
  (if (`self.Active`)
    (if (select `/Game/Blueprints/WindCurrent_Types` (`self.WindCurrentType`) :`NewEnumerator3` true)
      (for _array_element (`PrimitiveComponent.GetOverlappingActors` (`self.Box`) "/Game/Blueprints/Entities/Entity_BP.Entity_BP_C")
        (bind _asentity_bp (cast `/Game/Blueprints/Entities/Entity_BP` _array_element))
        (cast `/Game/Blueprints/Entities/TemperatureEntity_BP` _asentity_bp
          (:`CastFailed`
            (bind _box (`/Game/Blueprints/Entities/Entity_BP.Box` _asentity_bp))
            (if (`SceneComponent.IsSimulatingPhysics` _box "None")
              (if (`PrimitiveComponent.IsGravityEnabled` _box)
                (`PrimitiveComponent.SetEnableGravity` _box false)
                (`KismetSystemLibrary.PrintString` "GRAVITY OFF" true true (struct :`R` 1.0 :`B` 0.75 :`A` 1.0))))))))))

(event `self.Box.OnComponentBeginOverlap`
  (params (OverlappedComponent :type "PrimitiveComponent Object Reference") (OtherActor :type "Actor Object Reference") (OtherComp :type "PrimitiveComponent Object Reference") (OtherBodyIndex :type Integer) (bFromSweep :type Boolean) (SweepResult :type "HitResult Structure (by ref)"))
  (if (`self.Active`)
    (if (select `/Game/Blueprints/WindCurrent_Types` (`self.WindCurrentType`) :`NewEnumerator3` true)
      (bind _asentity_bp (cast `/Game/Blueprints/Entities/Entity_BP` OtherActor))
      (cast `/Game/Blueprints/Entities/TemperatureEntity_BP` _asentity_bp
        (:`CastFailed`
          (bind _box (`/Game/Blueprints/Entities/Entity_BP.Box` _asentity_bp))
          (if (`SceneComponent.IsSimulatingPhysics` _box "None")
            (if (`PrimitiveComponent.IsGravityEnabled` _box)
              (`PrimitiveComponent.SetEnableGravity` _box false)
              (`PrimitiveComponent.AddImpulse` _box (0.0 0.0 0.0) "None" true)
              (`KismetSystemLibrary.PrintString` "GRAVITY OFF" true true (struct :`R` 1.0 :`B` 0.75 :`A` 1.0)))))))))

(event `self.Box.OnComponentEndOverlap`
  (params (OverlappedComponent :type "PrimitiveComponent Object Reference") (OtherActor :type "Actor Object Reference") (OtherComp :type "PrimitiveComponent Object Reference") (OtherBodyIndex :type Integer))
  (if (select `/Game/Blueprints/WindCurrent_Types` (`self.WindCurrentType`) :`NewEnumerator3` true)
    (bind _asentity_bp (cast `/Game/Blueprints/Entities/Entity_BP` OtherActor))
    (cast `/Game/Blueprints/Entities/TemperatureEntity_BP` _asentity_bp
      (:`CastFailed`
        (bind _box (`/Game/Blueprints/Entities/Entity_BP.Box` _asentity_bp))
        (if (`SceneComponent.IsSimulatingPhysics` _box "None")
          (if (not (`PrimitiveComponent.IsGravityEnabled` _box))
            (`PrimitiveComponent.SetEnableGravity` _box true)
            (`KismetSystemLibrary.PrintString` "GRAVITY ON" true true (struct :`R` 1.0 :`B` 0.75 :`A` 1.0))))))))

(event `SetActiveVisuals`
  (bind _active (`self.Active`))
  (`SceneComponent.SetVisibility` (`self.Niagara`) _active false)
  (if _active
    _
    (elif (select `/Game/Blueprints/WindCurrent_Types` (`self.WindCurrentType`) :`NewEnumerator3` true)
      (for _array_element (`PrimitiveComponent.GetOverlappingActors` (`self.Box`) "/Game/Blueprints/Entities/Entity_BP.Entity_BP_C")
        (bind _asentity_bp (cast `/Game/Blueprints/Entities/Entity_BP` _array_element))
        (cast `/Game/Blueprints/Entities/TemperatureEntity_BP` _asentity_bp
          (:`CastFailed`
            (bind _box (`/Game/Blueprints/Entities/Entity_BP.Box` _asentity_bp))
            (if (`SceneComponent.IsSimulatingPhysics` _box "None")
              (if (not (`PrimitiveComponent.IsGravityEnabled` _box))
                (`PrimitiveComponent.SetEnableGravity` _box true)
                (`KismetSystemLibrary.PrintString` "GRAVITY ON" true true (struct :`R` 1.0 :`B` 0.75 :`A` 1.0))))))))))

(fn `UserConstructionScript`
  (`parent.UserConstructionScript`)
  (`SceneComponent.SetVisibility` (`self.Arrow`) (select `/Game/Blueprints/WindCurrent_Types` (`self.WindCurrentType`) :`NewEnumerator1` true :`NewEnumerator2` true) false))