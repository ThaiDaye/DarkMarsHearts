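; Short-lived spark entity that ignites other entities within its sphere.
; Shortly after BeginPlay it applies SparkIgnite to entities already overlapping the sphere, and later overlaps ignite on entry.
; A looping timer steadily drains its durability without shake, which appears to serve as its lifetime.
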(event `self.ReceiveBeginPlay`
  (`parent.ReceiveBeginPlay`)
  (`KismetSystemLibrary.K2_SetTimerDelegate` (delegate `TickCount`) 0.1 true)
  (`KismetSystemLibrary.Delay` 0.2)
  (for _array_element (`PrimitiveComponent.GetOverlappingActors` (`self.Sphere`) "/Game/Blueprints/Entities/Entity_BP.Entity_BP_C")
    (`self.SparkIgnite` _array_element)))

(event `TickCount`
  (`self.ReduceDurability` 1.0 false true))

(event `self.Sphere.OnComponentBeginOverlap`
  (params (OverlappedComponent :type "PrimitiveComponent Object Reference") (OtherActor :type "Actor Object Reference") (OtherComp :type "PrimitiveComponent Object Reference") (OtherBodyIndex :type Integer) (bFromSweep :type Boolean) (SweepResult :type "HitResult Structure (by ref)"))
  (`self.SparkIgnite` OtherActor))

(fn `UserConstructionScript`
  (`parent.UserConstructionScript`))