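; Temperature zone entity that spreads its temperature to entities inside its box and tints post-process white balance to match.
; On BeginPlay, a main zone sets overlapping entities' starting temperature, skipping other temperature zones.
; A one-second timer, while active, calls EmitTemperature immediately for entities near the player and staggers distant ones through a delayed-loop macro, guarded against overlapping passes.
; The construction script and BeginPlay refresh the post-process.
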(event `self.ReceiveBeginPlay`
  (`parent.ReceiveBeginPlay`)
  (`KismetSystemLibrary.K2_SetTimerDelegate` (delegate `TickEmitTemperature`) 1.0 true)
  (`self.SetTempPostProcess`)
  (for _array_element (`PrimitiveComponent.GetOverlappingActors` (`self.Box`) "/Game/Blueprints/Entities/Entity_BP.Entity_BP_C")
    (if (`self.MainTemperatureZone`)
      (cast `/Game/Blueprints/Entities/TemperatureEntity_BP` _array_element
        (:`CastFailed`
          (bind _asentity_bp (cast `/Game/Blueprints/Entities/Entity_BP` _array_element))
          (set `/Game/Blueprints/Entities/Entity_BP.Temperature` (`self.Temperature`) _asentity_bp))))))

(event `TickEmitTemperature`
  (bind _overlappingactors (`PrimitiveComponent.GetOverlappingActors` (`self.Box`) "/Game/Blueprints/Entities/Entity_BP.Entity_BP_C"))
  (set `self.InteractingUnits` (`KismetArrayLibrary.Array_Length` _overlappingactors))
  (if (== (`self.InteractingUnits`) 0)
    _
    (elif (`self.Active`)
      (for _array_element _overlappingactors
        (if (<= (`KismetMathLibrary.VSize` (- (`self.K2_GetActorLocation` _array_element) (`self.K2_GetActorLocation` (`self.PlayerRef`)))) 500.0)
          (cast `/Game/Blueprints/Entities/TemperatureEntity_BP` _array_element
            (:`CastFailed`
              (`self.EmitTemperature` (cast `/Game/Blueprints/Entities/Entity_BP` _array_element :!pure true) 1.0)))))
      (if (`self.TempUpdateFinished`)
        (set `self.TempUpdateFinished` false)
        (bind _newparam5 (`self.ForEachLoopDelay` _overlappingactors 0.0005)
          (:`NewParam4`
            (if (>= (`KismetMathLibrary.VSize` (- (`self.K2_GetActorLocation` _newparam5) (`self.K2_GetActorLocation` (`self.PlayerRef`)))) 500.0)
              (cast `/Game/Blueprints/Entities/TemperatureEntity_BP` _newparam5
                (:`CastFailed`
                  (`self.EmitTemperature` (cast `/Game/Blueprints/Entities/Entity_BP` _newparam5 :!pure true) 1.0)))))
          (:`NewParam7`
            (set `self.TempUpdateFinished` true)))))))

(fn `SetTempPostProcess`
  (set `PostProcessComponent.Settings` (make `PostProcessSettings` :`WhiteTemp` (select `bool` (`self.Active`) :`false` 6500.0 :`true` (+ (`KismetMathLibrary.FClamp` (* (+ (`self.Temperature`) 80.0) 50.0) 2000.0 13500.0) 1500.0))) (`self.PostProcess`)))

(fn `UserConstructionScript`
  (`parent.UserConstructionScript`)
  (`self.SetTempPostProcess`))