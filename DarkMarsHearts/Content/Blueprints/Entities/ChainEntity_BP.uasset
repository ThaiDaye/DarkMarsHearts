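; Chain entity that tethers a Host entity to a Target entity with a physics constraint and a visible cable.
; On BeginPlay it attaches to the Host, registers in both entities' ChainRef lists and fires GrabEvent on any AI endpoint.
; It destroys itself if either end is liquid.
; A fast looping timer also destroys it when either end is invalid or Host, Target or chain Durability hits zero.
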(event `DestroyOnDurabilityLost`
  (bind _target (`self.Target`))
  (bind _host (`self.Host`))
  (`|ExecutionSequence`
    (:`then_0`
      (`/Engine/EditorBlueprintResources/StandardMacros.IsValid` _host
        (:`Is Valid`
          (if (== (`/Game/Blueprints/Entities/Entity_BP.Durability` _host) 0.0)
            (`self.K2_DestroyActor` :!label _label)))
        (:`Is Not Valid`
          (goto _label))))
    (:`then_1`
      (`/Engine/EditorBlueprintResources/StandardMacros.IsValid` _target
        (:`Is Valid`
          (if (== (`/Game/Blueprints/Entities/Entity_BP.Durability` _target) 0.0)
            (goto _label)
            (elif (== (`self.Durability`) 0.0)
              (goto _label))))
        (:`Is Not Valid`
          (goto _label))))))

(event `self.ReceiveDestroyed`
  (bind _target (`self.Target`))
  (bind _host (`self.Host`))
  (`/Engine/EditorBlueprintResources/StandardMacros.IsValid` _host
    (:`Is Valid`
      (`KismetArrayLibrary.Array_RemoveItem` (`/Game/Blueprints/Entities/Entity_BP.ChainRef` _host) self))
    (:`Is Not Valid`
      _))
  (`/Engine/EditorBlueprintResources/StandardMacros.IsValid` _target
    (:`Is Valid`
      (`KismetArrayLibrary.Array_RemoveItem` (`/Game/Blueprints/Entities/Entity_BP.ChainRef` _target) self))
    (:`Is Not Valid`
      _))
  (`self.DestroyOnDurabilityLost`))

(event `SetChain`
  (bind _host (`self.Host`))
  (bind _target (`self.Target`))
  (bind _host_2 (`self.Host`))
  (`/Engine/EditorBlueprintResources/StandardMacros.IsValid` (`self.Host`)
    (:`Is Valid`
      (`/Engine/EditorBlueprintResources/StandardMacros.IsValid` (`self.Target`)
        (:`Is Valid`
          (`SceneComponent.K2_SetWorldLocation` (`self.Box`) (`self.K2_GetActorLocation` _host_2) false false :!label _label_2)
          (cast `/Game/Blueprints/Entities/LiquidEntity_BP` _host_2
            (:`then`
              (`self.K2_DestroyActor` :!label _label_3))
            (:`CastFailed`
              (cast `/Game/Blueprints/Entities/LiquidEntity_BP` (`self.Target`)
                (:`then`
                  (goto _label_3))
                (:`CastFailed`
                  (`self.K2_AttachToActor` _host_2 "None" "KeepWorld" "KeepWorld" "KeepWorld")
                  (`KismetArrayLibrary.Array_Add` (`/Game/Blueprints/Entities/Entity_BP.ChainRef` _host) self)
                  (`KismetArrayLibrary.Array_Add` (`/Game/Blueprints/Entities/Entity_BP.ChainRef` _target) self)
                  (`PhysicsConstraintComponent.SetConstrainedComponents` (`self.PhysicsConstraint`) (`/Game/Blueprints/Entities/Entity_BP.Box` _host) "None" (`/Game/Blueprints/Entities/Entity_BP.Box` _target) "None")
                  (`CableComponent.SetAttachEndTo` (`self.Cable`) (`self.Target`) "Box" "None")
                  (set `/Game/Blueprints/Entities/Entity_BP.ChainAnchorRef` true _host)
                  (`|ExecutionSequence`
                    (:`then_0`
                      (bind _asai_entity_bp (cast `/Game/Blueprints/Entities/AiEntity_BP` _host))
                      (`/Game/Blueprints/Entities/AiEntity_BP.GrabEvent` _asai_entity_bp))
                    (:`then_1`
                      (bind _asai_entity_bp_2 (cast `/Game/Blueprints/Entities/AiEntity_BP` _target))
                      (`/Game/Blueprints/Entities/AiEntity_BP.GrabEvent` _asai_entity_bp_2))))))))))))

(event `self.ReceiveBeginPlay`
  (`parent.ReceiveBeginPlay`)
  (`KismetSystemLibrary.K2_SetTimerDelegate` (delegate `DestroyOnDurabilityLost`) 0.05 true)
  (goto _label_2))

(fn `UserConstructionScript`
  (`parent.UserConstructionScript`))