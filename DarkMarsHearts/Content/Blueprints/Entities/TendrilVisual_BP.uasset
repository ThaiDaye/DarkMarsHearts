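; TendrilVisual_BP is an entity Blueprint that visualizes a tendril with a CableComponent, configured by collision, gravity, length and force variables.
; The construction script and BeginPlay both apply collision, length and a gravity toggle that picks either a very faint or zero gravity scale.
; A looping timer periodically sets the cable force along the Arrow's forward vector, scaled by Force, so changes in arrow direction are picked up only at each interval.
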(event `self.ReceiveBeginPlay`
  (bind _cablecomponent (`self.CableComponent`))
  (set `CableComponent.bEnableCollision` (`self.Collisions`) (`self.CableComponent`))
  (`KismetSystemLibrary.K2_SetTimerDelegate` (delegate `UdpateForce`) 5.0 true)
  (set `CableComponent.CableGravityScale` (select `bool` (`self.Gravity`) :`true` 0.01 :!type "Float (single-precision)") _cablecomponent)
  (set `CableComponent.CableLength` (`self.Length`) _cablecomponent))

(event `UdpateForce`
  (set `CableComponent.CableForce` (* (`SceneComponent.GetForwardVector` (`self.Arrow`)) (`self.Force`)) (`self.CableComponent`)))

(fn `UserConstructionScript`
  (bind _cablecomponent (`self.CableComponent`))
  (set `CableComponent.bEnableCollision` (`self.Collisions`) (`self.CableComponent`))
  (set `CableComponent.CableGravityScale` (select `bool` (`self.Gravity`) :`true` 0.01 :!type "Float (single-precision)") _cablecomponent)
  (set `CableComponent.CableLength` (`self.Length`) _cablecomponent))