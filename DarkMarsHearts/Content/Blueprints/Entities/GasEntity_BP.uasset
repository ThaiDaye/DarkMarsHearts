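; Gas cloud entity that expands over time and decays, with a type such as smoke, hydrogen or steam.
; Looping timers grow its collision sphere, reduce durability, and drive Niagara radius, size, spawn count and fade.
; A larger or more durable cloud absorbs an overlapping same-type gas, gaining durability and destroying the other.
; Steam wets non-temperature entities on overlap and periodically while they stay inside, scaled by durability.
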(event `TickCount`
  (`NiagaraComponent.SetNiagaraVariableInt` (`self.GasParticle`) "User.Spawn Count" (`KismetMathLibrary.FTrunc` (`KismetMathLibrary.Lerp` 0.0 50.0 (/ (`self.Durability`) (`self.MaxDurability`)))))
  (`self.ReduceDurability` (`self.DecayRate`) false true))

(event `Tick Size`
  (bind _gasradiusmax (`self.GasRadiusMax`))
  (bind _gasradius (`self.GasRadius`))
  (bind _gasparticle (`self.GasParticle`))
  (bind _returnvalue (`KismetMathLibrary.FClamp` (+ _gasradius (+ (* (/ (`KismetMathLibrary.FClamp` _gasradius 1.0 500.0) 500.0) 10.0) 5.0)) 0.0 (select `bool` (== _gasradiusmax 0.0) :`false` _gasradiusmax :`true` 500.0)))
  (bind _output_get (set `self.GasRadius` _returnvalue))
  (bind _returnvalue_2 (+ _output_get (* (`self.MaxDurability`) 0.5)))
  (`SphereComponent.SetSphereRadius` (`self.Sphere`) (+ _returnvalue_2 -20.0) true)
  (`NiagaraComponent.SetNiagaraVariableFloat` _gasparticle "User.GasRadius" _returnvalue_2)
  (`NiagaraComponent.SetNiagaraVariableFloat` (`self.GasParticle`) "User.GasSize" (* _returnvalue 0.1))
  (`NiagaraComponent.SetNiagaraVariableFloat` _gasparticle "User.GasFade" (* (`self.GasOpacity`) (`KismetMathLibrary.Lerp` 0.0 1.0 (/ (`self.Durability`) (`self.MaxDurability`))))))

(event `self.ReceiveBeginPlay`
  (bind _gasparticle (`self.GasParticle`))
  (`parent.ReceiveBeginPlay`)
  (set `self.Name` (`KismetStringLibrary.Concat_StrStr` "Gas " (`|GetEnumeratorNameAsString` (`self.GasType`)) " Entity"))
  (`self.Tick Size`)
  (`self.TickCount`)
  (`KismetSystemLibrary.K2_SetTimerDelegate` (delegate `Tick Size`) (`self.GasExpandRate`) true)
  (`KismetSystemLibrary.K2_SetTimerDelegate` (delegate `TickCount`) 1.0 true)
  (`KismetSystemLibrary.K2_SetTimerDelegate` (delegate `WetFromSteam`) 5.0 true)
  (`NiagaraComponent.SetNiagaraVariableVec3` _gasparticle "User.GasColour" (`KismetMathLibrary.Conv_LinearColorToVector` (`self.GasColour`)))
  (`NiagaraComponent.SetNiagaraVariableVec3` _gasparticle "User.GasSubColour" (`KismetMathLibrary.Conv_LinearColorToVector` (`self.GasSubColour`))))

(event `WetFromSteam`
  (bind _sphere (`self.Sphere`))
  (bind _gastype (`self.GasType`))
  (bind _overlappingactors (`PrimitiveComponent.GetOverlappingActors` _sphere "/Game/Blueprints/Entities/Entity_BP.Entity_BP_C"))
  ;[1 1 1] wet froms team (passive
  (if (`|EnumEquality` _gastype "NewEnumerator4")
    (`/Engine/EditorBlueprintResources/StandardMacros.IsValid` _sphere
      (:`Is Valid`
        (if (> (`KismetArrayLibrary.Array_Length` _overlappingactors) 0)
          (for _array_element _overlappingactors
            (if (not (== _array_element self))
              (bind _asentity_bp (cast `/Game/Blueprints/Entities/Entity_BP` _array_element))
              (cast `/Game/Blueprints/Entities/TemperatureEntity_BP` _array_element
                (:`CastFailed`
                  (`self.ApplyWetness` _asentity_bp (* (`self.Durability`) 0.0001) false (select `/Game/Blueprints/P_Gas_Types` _gastype :`NewEnumerator0` "NewEnumerator0" :`NewEnumerator1` "NewEnumerator0" :`NewEnumerator2` "NewEnumerator0" :`NewEnumerator4` "NewEnumerator1" :`NewEnumerator5` "NewEnumerator4" :!type "/Game/Blueprints/P_Liquid_Types Enum"))
                  (`KismetSystemLibrary.PrintString` "WET FROM STEAM (PASSIVE)" true true (struct :`G` 0.342126 :`B` 1.0 :`A` 1.0)))))))))))

(event `self.Sphere.OnComponentBeginOverlap`
  (params (OverlappedComponent :type "PrimitiveComponent Object Reference") (OtherActor :type "Actor Object Reference") (OtherComp :type "PrimitiveComponent Object Reference") (OtherBodyIndex :type Integer) (bFromSweep :type Boolean) (SweepResult :type "HitResult Structure (by ref)"))
  (bind _gastype (`self.GasType`))
  ;[1 1 1] wet from steam & gas combine
  (bind _asentity_bp (cast `/Game/Blueprints/Entities/Entity_BP` OtherActor))
  (bind _asgas_entity_bp (cast `/Game/Blueprints/Entities/GasEntity_BP` OtherActor)
    (:`then`
      (if (`|EnumEquality` (`/Game/Blueprints/Entities/GasEntity_BP.GasType` _asgas_entity_bp) (`self.GasType`))
        (if (== OtherComp (`/Game/Blueprints/Entities/Entity_BP.Box` _asgas_entity_bp))
          (`/Engine/EditorBlueprintResources/StandardMacros.IsValid` _asgas_entity_bp
            (:`Is Valid`
              (if (> (`self.MaxDurability`) (`/Game/Blueprints/Entities/Entity_BP.MaxDurability` _asgas_entity_bp))
                (bind _durability (`/Game/Blueprints/Entities/Entity_BP.Durability` _asgas_entity_bp))
                (`self.ReduceDurability` (* _durability -2.0) false true true :!label _label)
                (`KismetSystemLibrary.PrintString` "GAS COMBINE" true true (struct :`R` 0.071088 :`G` 1.0 :`A` 1.0))
                (`self.K2_DestroyActor` _asgas_entity_bp)
                (elif (> (`self.Durability`) _durability)
                  (goto _label))))))))
    (:`CastFailed`
      (cast `/Game/Blueprints/Entities/TemperatureEntity_BP` OtherActor
        (:`CastFailed`
          (if (`|EnumEquality` _gastype "NewEnumerator4")
            (`self.ApplyWetness` _asentity_bp (* (`self.Durability`) 0.001) false (select `/Game/Blueprints/P_Gas_Types` _gastype :`NewEnumerator0` "NewEnumerator0" :`NewEnumerator1` "NewEnumerator2" :`NewEnumerator2` "NewEnumerator0" :`NewEnumerator4` "NewEnumerator1" :`NewEnumerator5` "NewEnumerator4" :!type "/Game/Blueprints/P_Liquid_Types Enum"))
            (`KismetSystemLibrary.PrintString` "WET FROM STEAM" true true (struct :`G` 0.342126 :`B` 1.0 :`A` 1.0))))))))

(fn `UserConstructionScript`
  (bind _gasparticle (`self.GasParticle`))
  (`parent.UserConstructionScript`)
  (`NiagaraComponent.SetNiagaraVariableFloat` _gasparticle "User.GasFade" (`self.GasOpacity`))
  (`NiagaraComponent.SetNiagaraVariableVec3` _gasparticle "User.GasColour" (`KismetMathLibrary.Conv_LinearColorToVector` (`self.GasColour`)))
  (`NiagaraComponent.SetNiagaraVariableVec3` _gasparticle "User.GasSubColour" (`KismetMathLibrary.Conv_LinearColorToVector` (`self.GasSubColour`))))