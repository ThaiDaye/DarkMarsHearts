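; Footprint entity that marks a spot on world geometry and wears away over time.
; On BeginPlay a sphere trace at its Box checks for WorldStatic surfaces and destroys the actor when none is hit.
; Otherwise it copies Temperature from its Host, if valid, and starts a looping one-second timer.
; Each DecayTick reduces durability by a random amount and destroys the actor once Durability reaches zero.
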(event `self.ReceiveBeginPlay`
  (bind _host (`self.Host`))
  (bind _returnvalue (`SceneComponent.K2_GetComponentLocation` (`self.Box`)))
  (`parent.ReceiveBeginPlay`)
  (bind _outhit (`KismetSystemLibrary.SphereTraceSingleForObjects` _returnvalue _returnvalue 25.0 (`|MakeArray` "ObjectTypeQuery1" :!type "EObjectTypeQuery Enum")))
  (if (`GameplayStatics.BreakHitResult` _outhit)
    (`KismetSystemLibrary.K2_SetTimerDelegate` (delegate `DecayTick`) 1.0 true)
    (`/Engine/EditorBlueprintResources/StandardMacros.IsValid` _host
      (:`Is Valid`
        (set `self.Temperature` (`/Game/Blueprints/Entities/Entity_BP.Temperature` _host))))
    (else
      (`self.K2_DestroyActor`))))

(event `DecayTick`
  (`self.ReduceDurability` (`KismetMathLibrary.RandomFloatInRange` 5.0 10.0))
  (if (== (`self.Durability`) 0.0)
    (`self.K2_DestroyActor`)))

(fn `UserConstructionScript`
  (`parent.UserConstructionScript`))